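; Gameplay ability that handles a character's death by playing a death montage and then destroying the avatar actor.
; On activation it stops the AI controller's brain logic, if present.
; It queries the avatar's combat component interface by the Death gameplay tag and plays a randomly picked montage and speed.
; Completion, blend out, interruption or cancellation all destroy the actor and end the ability.
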(event Ability|EventActivateAbility
  (bind _returnvalue (Ability|GetAvatarActorfromActorInfo))
  (bind _returnvalue_2 (AI|GetAIController _returnvalue))
  (bind _returnvalue_3 (Actor|GetComponentbyClass _returnvalue_2 "/Script/AIModule.BrainComponent"))
  (Utilities|IsValid _returnvalue_3
    (:Is%20Valid
      (AI|Logic|StopLogic _returnvalue_3 ""))
    (:Is%20Not%20Valid
      _))
  (bind _returnvalue_4 (Class|CombatComponentInterface|GetMontageAction(Message) (Utilities|Array|Get(acopy) (Class|Actor|GetComponentsbyInterface (Ability|GetAvatarActorfromActorInfo) "/Script/CombatAbilitiesSystem.CombatComponentInterface")) (GameplayTags|MakeLiteralGameplayTag "(TagName=\"CombatAbilities.Death\")")))
  (|PlayMontageandWaitforEvent :MontageToPlay (.Montage (Utilities|Struct|BreakCombatAnimationInfo (.OutItem (Utilities|Array|Random _returnvalue_4)))) :Rate (.Speed (Utilities|Struct|BreakCombatAnimationInfo (.OutItem (Utilities|Array|Random _returnvalue_4))))
    (:OnCompleted
      _)
    (:OnBlendOut
      _)
    (:OnInterrupted
      _)
    (:OnCancelled
      _))
  (Actor|DestroyActor (Ability|GetAvatarActorfromActorInfo))
  (Ability|EndAbility))